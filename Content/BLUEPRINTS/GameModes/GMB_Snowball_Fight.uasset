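; Game mode for the snowball fight that runs a start countdown before play begins.
; BeginPlay shows the countdown widget, pauses the AI's brain logic and player input, then after the countdown delay restores both, removes the widget and reveals the game UI.
; A one-second Delay on Tick paces the countdown, playing a sound per step and a whoosh at zero.
; A start screen widget is created but not displayed here.
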(event EventTick
  (params (DeltaSeconds :type Float%20%28single-precision%29))
  ;[0.15 0.15 0.15 0.5] Countdown to game start
  (Utilities|FlowControl|Delay 1.0)
  (if (== (Variables|Default|GetCurrent%20Countdown) 0)
    (Utilities|FlowControl|DoOnce false
      (:Completed
        (Audio|PlaySound2D "/Game/ASSETS/Audio/Sound_Effects/Cues/Whoosh_Sound_Cue.Whoosh_Sound_Cue" 1.0 1.0 0.0 0 0)))
    (else
      (Variables|Default|SetCurrent%20Countdown (Math|Integer|Clamp(Integer) (- (Variables|Default|GetCurrent%20Countdown) 1) 0 (Variables|Default|GetCountdown%20Max)))
      (Audio|PlaySound2D "/Game/ASSETS/Audio/Sound_Effects/Cues/Start_Sound_Cue.Start_Sound_Cue" 1.0 1.0 0.0 0 0))))

(event EventBeginPlay
  (Utilities|FlowControl|Sequence
    (:then_0
      ;[0.15 0.15 0.15 0.5] Reference start screen widget
      (bind _returnvalue (UserInterface|CreateWidget "/Game/WIDGETS/GameUI/WBP_CountdownToStart.WBP_CountdownToStart_C"))
      (bind _output_get (Variables|Default|SetCountdown%20Widget%20REF _returnvalue))
      (UserInterface|Viewport|AddtoViewport _output_get 0)
      ;[0.15 0.15 0.15 0.5] Reference Start Widget
      (bind _returnvalue_2 (UserInterface|CreateWidget "/Game/WIDGETS/GameUI/WBP_StartScreen.WBP_StartScreen_C"))
      (Variables|Default|SetStart%20Widget%20REF _returnvalue_2))
    (:then_1
      ;[0.15 0.15 0.15 0.5] Disable both AI and player controllers logics
      (bind _returnvalue_3 (Actor|GetActorOfClass "/Game/BLUEPRINTS/AICharacter/BP_AI_Character.BP_AI_Character_C"))
      (bind _asbp_ai_controller (Utilities|Casting|CastToBP_AI_Controller (AI|GetAIController _returnvalue_3)))
      (AI|Logic|StopLogic (Variables|/Script/AIModule.AIController|GetBrainComponent _asbp_ai_controller) "Waiting To Start")
      (Input|DisableInput (Game|GetPlayerCharacter 0) (Game|GetPlayerController 0))
      ;[0.15 0.15 0.15 0.5] Delay by countdown amount
      (Utilities|FlowControl|Delay (Math|Conversions|ToFloat(Integer) (Variables|Default|GetCountdown%20Max)))
      ;[0.15 0.15 0.15 0.5] Start AI and Player controllers logics
      (bind _returnvalue_4 (Actor|GetActorOfClass "/Game/BLUEPRINTS/AICharacter/BP_AI_Character.BP_AI_Character_C"))
      (bind _asbp_ai_controller_2 (Utilities|Casting|CastToBP_AI_Controller (AI|GetAIController _returnvalue_4)))
      (AI|Logic|StartLogic (Variables|/Script/AIModule.AIController|GetBrainComponent _asbp_ai_controller_2))
      (Input|EnableInput (Game|GetPlayerCharacter 0) (Game|GetPlayerController 0))
      (Widget|RemovefromParent (Variables|Default|GetCountdown%20Widget%20REF))
      ;[0.15 0.15 0.15 0.5] Display Game UI
      (bind _returnvalue_5 (Actor|GetActorOfClass "/Game/BLUEPRINTS/Managers/BP_GameUI_Manager.BP_GameUI_Manager_C"))
      (bind _output_get_2 (Variables|Default|SetGameUI%20REF _returnvalue_5))
      (Widget|SetVisibility (Variables|/Game/BLUEPRINTS/Managers/BP_GameUI_Manager.BP_GameUI_Manager_C|GetGameUI%20REF _output_get_2) "Visible")
      (Utilities|Time|ClearandInvalidateTimerbyHandle (Variables|Default|GetTimer%20HDL)))))

(fn ConstructionScript)