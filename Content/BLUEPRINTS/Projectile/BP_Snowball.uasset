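; BP_Snowball is a projectile that can be launched at an optional target and bursts on impact.
; Construction applies Speed and Gravity to its ProjectileMovement; BeginPlay ignores collision with the owner and aims the velocity at any valid Target once, without homing.
; On hit it calls OnImpact, plays snow sound and Niagara burst, destroys itself, and calls OnPlayerHit if it struck the player character.
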(event OnComponentHit(Collider)
  (params (HitComponent :type Primitive%20Component%20Object%20Reference) (OtherActor :type Actor%20Object%20Reference) (OtherComp :type Primitive%20Component%20Object%20Reference) (NormalImpulse :type Vector :default "0, 0, 0") (Hit :type Hit%20Result%20Structure%20%28by%20ref%29))
  (bind (_bblockinghit _binitialoverlap _time _distance _location _impactpoint _normal _impactnormal _physmat _hitactor) (Collision|BreakHitResult Hit))
  ;[0.15 0.15 0.15 0.5] Snowball impact logic
  (Default|CallOnImpact OtherActor Hit)
  (Audio|PlaySoundatLocation "/Game/ASSETS/Audio/Sound_Effects/Cues/snow_impact_Cue.snow_impact_Cue" _location "0, 0, 0" 1.0 1.0 0.0 0 0 0 0)
  (Niagara|SpawnSystematLocation "/Game/BLUEPRINTS/Projectile/NS_Snow_Burst.NS_Snow_Burst" _location)
  (Utilities|FlowControl|Sequence
    (:then_0
      (Actor|DestroyActor))
    (:then_1
      ;[0.15 0.15 0.15 0.5] Send a signal if player is the one taking hit
      (if (== (Game|GetPlayerCharacter 0) _hitactor)
        (Default|CallOnPlayerHit)))))

(event Custom|Rotate%20To%20Target
  ;[0.15 0.15 0.15 0.5] Function to launch towards a target
  (Variables|/Script/Engine.MovementComponent|SetVelocity (Variables|Default|GetProjectileMovement) (* (Math|Vector|GetUnitDirection(Vector) (Transformation|GetActorLocation) (Transformation|GetActorLocation (Variables|Settings|GetTarget))) (Variables|Settings|GetSpeed))))

(event EventBeginPlay
  ;[0.15 0.15 0.15 0.5] Ignore collision with whatever spawns the snowball
  (Collision|IgnoreActorwhenMoving (Variables|Default|GetCollider) (Components|GetOwner) true)
  ;[0.15 0.15 0.15 0.5] Rotate to target if applicable
  (Variables|Settings|GetTarget
    (:then
      (CallFunction|RotatetoTarget))
    (:else)))

(fn ConstructionScript
  (bind _projectilemovement (Variables|Default|GetProjectileMovement))
  ;[0.15 0.15 0.15 0.5] Construction logic
  (Variables|/Script/Engine.ProjectileMovementComponent|SetInitialSpeed _projectilemovement (Variables|Settings|GetSpeed))
  (Variables|/Script/Engine.ProjectileMovementComponent|SetMaxSpeed _projectilemovement (Variables|Settings|GetSpeed))
  (Variables|/Script/Engine.ProjectileMovementComponent|SetProjectileGravityScale _projectilemovement (Variables|Settings|GetGravity)))