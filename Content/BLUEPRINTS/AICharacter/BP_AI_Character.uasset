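; BP_AI_Character is the AI child opponent in a snowball fight, throwing snowballs at the player and taking hits.
; Projectile hits play random reactions, report damage to AI perception and apply damage, which updates the game UI's health values.
; At zero health it stops AI logic and movement and flags game over in the game instance.
; Helpers supply randomized attack/defend ranges and state-based walk speeds; dispatchers signal damage taken and attack end.
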(event Custom|Throw%20Snowball
  ;[0.15 0.15 0.15 0.5] Throw Snowball (Attack)
  (Utilities|FlowControl|Sequence
    (:then_0
      (Utilities|FlowControl|Delay 0.5)
      (bind _returnvalue (Game|SpawnActorfromClass "/Game/BLUEPRINTS/Projectile/BP_Snowball.BP_Snowball_C" (Transformation|GetWorldTransform (Variables|Default|GetSnowlaunch%20Point)) "Undefined" "MultiplyWithRoot" 0 4e+03 1.0 (Game|GetPlayerCharacter 0) 0))
      (Collision|IgnoreActorwhenMoving (Variables|/Game/BLUEPRINTS/Projectile/BP_Snowball.BP_Snowball_C|GetCollider _returnvalue) self true)
      (Default|RotatetoTarget _returnvalue)
      (EventDispatchers|AssignOnPlayerHit _returnvalue (delegate Custom|Happy%20Dialogue)))
    (:then_1
      (bind _returnvalue_2 (Animation|PlayAnimMontage "/Game/ASSETS/Animations/Player/Throw_Ball_Montage.Throw_Ball_Montage" 1.0 "None"))
      (Utilities|FlowControl|Delay _returnvalue_2)
      (Default|CallOnAttackEnd))))

(event Custom|Happy%20Dialogue
  ;[0.15 0.15 0.15 0.5] Throw Snowball (Attack)
  (Utilities|FlowControl|Delay 0.75)
  (Audio|PlaySoundatLocation "/Game/ASSETS/Audio/Dialogues/Player_and_AI/Boy_DealsDamage_Dialogue_CUE.Boy_DealsDamage_Dialogue_CUE" (Transformation|GetActorLocation) "0, 0, 0" 1.0 1.0 0.0 0 0 0 0))

(event Collision|EventHit
  (params (MyComp :type Primitive%20Component%20Object%20Reference) (Other :type Actor%20Object%20Reference) (OtherComp :type Primitive%20Component%20Object%20Reference) (bSelfMoved :type Boolean) (HitLocation :type Vector :default "0, 0, 0") (HitNormal :type Vector :default "0, 0, 0") (NormalImpulse :type Vector :default "0, 0, 0") (Hit :type Hit%20Result%20Structure%20%28by%20ref%29))
  (bind _returnvalue (Game|GetPlayerCharacter 0))
  (bind _montage_to_play (Variables|Default|GetMontage%20To%20Play))
  ;[0.15 0.15 0.15 0.5] AI hit feedback
  (if (Utilities|DoesObjectImplementInterface Other "/Game/BLUEPRINTS/Projectile/BPI_Projectile.BPI_Projectile_C")
    (Animation|PlayAnimMontage (Utilities|Array|Get(acopy) _montage_to_play (Math|Random|RandomInteger (Utilities|Array|Length _montage_to_play))) 1.0 "None")
    (Audio|PlaySoundatLocation "/Game/ASSETS/Audio/Dialogues/Player_and_AI/Boy_ReceivesDamage_Dialogue_CUE.Boy_ReceivesDamage_Dialogue_CUE" (Transformation|GetActorLocation) "0, 0, 0" 1.0 1.0 0.0 0 0 0 0)
    (Class|AISenseDamage|ReportDamageEvent self _returnvalue 1.0 (Transformation|GetActorLocation _returnvalue) "0, 0, 0" "None")
    (Game|Damage|ApplyDamage self 1.0 0 0 "/Script/Engine.DamageType")
    (Default|CallOnDamageTaken)))

(event Game|Damage|EventAnyDamage
  (params (Damage :type Float%20%28single-precision%29) (DamageType :type Damage%20Type%20Object%20Reference) (InstigatedBy :type Controller%20Object%20Reference) (DamageCauser :type Actor%20Object%20Reference))
  ;[0.15 0.15 0.15 0.5] AI Health Damage
  (if (not (Variables|Default|GetIs%20Dead?))
    (bind _output_get (Variables|Default|SetCurrent%20Health (Math|Float|Clamp(Float) (- (Variables|Default|GetCurrent%20Health) Damage) 0.0 (Variables|Default|GetMax%20Health))))
    (bind _output_get_2 (Variables|/Game/WIDGETS/GameUI/WBP_GameUI.WBP_GameUI_C|SetCurrent%20AI%20Health (Variables|/Game/BLUEPRINTS/Managers/BP_GameUI_Manager.BP_GameUI_Manager_C|GetGameUI%20REF (Variables|Default|GetGameUI%20Manager)) _output_get))
    ;[0.15 0.15 0.15 0.5] Check health status
    (if (<= _output_get_2 0.0)
      (Utilities|FlowControl|Sequence
        (:then_0
          ;[0.15 0.15 0.15 0.5] AI Death
          (Variables|Default|SetIs%20Dead? true)
          (Audio|PlaySound2D "/Game/ASSETS/Audio/Dialogues/Player_and_AI/Child_sobbing_Cue.Child_sobbing_Cue" 1.0 1.0 0.0 0 0)
          (bind _asbp_ai_controller (Utilities|Casting|CastToBP_AI_Controller (AI|GetAIController self)))
          (AI|Logic|StopLogic (Variables|/Script/AIModule.AIController|GetBrainComponent _asbp_ai_controller) "Dead")
          (Pawn|Components|CharacterMovement|DisableMovement (Variables|Character|GetCharacterMovement)))
        (:then_1
          ;[0.15 0.15 0.15 0.5] Set 'Game Over' to TRUE
          (bind _asbp_game_instance (Utilities|Casting|CastToBP_GameInstance (Game|GetGameInstance)))
          (Variables|/Game/BLUEPRINTS/GameInstance/BP_GameInstance.BP_GameInstance_C|SetIs%20Game%20Over? _asbp_game_instance true))))))

(event EventBeginPlay
  ;[0.15 0.15 0.15 0.5] Reference Game UI Manager
  (bind _returnvalue (Actor|GetActorOfClass "/Game/BLUEPRINTS/Managers/BP_GameUI_Manager.BP_GameUI_Manager_C"))
  (bind _output_get (Variables|Default|SetGameUI%20Manager _returnvalue))
  ;[0.15 0.15 0.15 0.5] Initialize AI's health
  (Variables|/Game/WIDGETS/GameUI/WBP_GameUI.WBP_GameUI_C|SetCurrent%20AI%20Health (Variables|/Game/BLUEPRINTS/Managers/BP_GameUI_Manager.BP_GameUI_Manager_C|GetGameUI%20REF _output_get) (Variables|Default|GetCurrent%20Health))
  (Variables|/Game/WIDGETS/GameUI/WBP_GameUI.WBP_GameUI_C|SetMax%20AI%20Health (Variables|/Game/BLUEPRINTS/Managers/BP_GameUI_Manager.BP_GameUI_Manager_C|GetGameUI%20REF _output_get) (Variables|Default|GetMax%20Health)))

(fn ConstructionScript)

(fn GetIdealRange
  (return (Math|Random|RandomFloatinRange 5e+02 7e+02) (Math|Random|RandomFloatinRange 8e+02 1e+03)))

(fn SetMovementSpeed
  (params (Movement%20Speed :type E_Movement_Speed%20Enum :default "NewEnumerator0"))
  ;[0.15 0.15 0.15 0.5] Set Movement Speed
  (bind _output_get (Variables|/Script/Engine.CharacterMovementComponent|SetMaxWalkSpeed (Variables|Character|GetCharacterMovement) (Utilities|Select :Index Movement%20Speed :NewEnumerator0 0.0 :NewEnumerator1 0.0 :NewEnumerator2 5e+02 :NewEnumerator3 7.5e+02 :NewEnumerator4 1e+03)))
  (return _output_get))