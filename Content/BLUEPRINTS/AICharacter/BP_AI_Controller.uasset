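; AI controller that runs an Easy, Medium or Hard behavior tree from the game instance's difficulty and seeds attack and defend radii from the possessed pawn.
; Perception updates pass through per-sense handlers gated by the Blackboard state enum, which starts Passive.
; Seeing the player or taking damage can trigger Attacking with a target.
; Sound handling sets Investigating with a location, but its sense class is unset in CanSenseActor.
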(event OnPerceptionUpdated(AIPerception)
  (params (UpdatedActors :type Array%20of%20Actor%20Object%20References))
  ;[0.15 0.15 0.15 0.5] AI Perception Logic
  (for _array_element UpdatedActors
    (Utilities|FlowControl|Sequence
      (:then_0
        (bind _sensed (CallFunction|CanSenseActor _array_element "NewEnumerator1"))
        (if _sensed
          (CallFunction|HandleSensedSight _array_element)))
      (:then_1
        (bind (_sensed_2 _stimulus) (CallFunction|CanSenseActor _array_element "NewEnumerator3"))
        (if _sensed_2
          (CallFunction|HandleSensedSound (.StimulusLocation (Utilities|Struct|BreakAIStimulus _stimulus)))))
      (:then_2
        (bind _sensed_3 (CallFunction|CanSenseActor _array_element "NewEnumerator2"))
        (if _sensed_3
          (CallFunction|HandleSensedDamage _array_element))))))

(event EventPossess
  (params (PossessedPawn :type Pawn%20Object%20Reference))
  ;[0.15 0.15 0.15 0.5] Run Behaviour Tree based on difficulty
  (bind _asbp_game_instance (Utilities|Casting|CastToBP_GameInstance (Game|GetGameInstance)))
  (switch Utilities|FlowControl|Switch|SwitchonE_DifficultyModes (Variables|/Game/BLUEPRINTS/GameInstance/BP_GameInstance.BP_GameInstance_C|GetDifficulty%20Mode _asbp_game_instance)
    (:NewEnumerator0
      ;[0.15 0.15 0.15 0.5] Run BT and initial state
      (AI|RunBehaviorTree "/Game/BLUEPRINTS/AICharacter/AI_System/BT_AI_Easy.BT_AI_Easy"))
    (:NewEnumerator1
      (AI|RunBehaviorTree "/Game/BLUEPRINTS/AICharacter/AI_System/BT_AI_Medium.BT_AI_Medium"))
    (:NewEnumerator2
      (AI|RunBehaviorTree "/Game/BLUEPRINTS/AICharacter/AI_System/BT_AI_Hard.BT_AI_Hard")))
  (CallFunction|SetStateasPassive)
  ;[0.15 0.15 0.15 0.5] Set attack and defend radius
  (bind (_attack_radius _defend_radius) (Class|BPIAI|GetIdealRange(Message) PossessedPawn))
  (AI|Components|Blackboard|SetValueasFloat (Variables|Default|GetBlackboard) (Variables|Default|GetAttack%20Radius%20Key) _attack_radius)
  (AI|Components|Blackboard|SetValueasFloat (Variables|Default|GetBlackboard) (Variables|Default|GetDefend%20Radius%20Key) _defend_radius))

(fn ConstructionScript)

(fn GetCurrentState
  ;[0.15 0.15 0.15 0.5] Get current state
  (return (Utilities|Enum|ByteToEnumE_AI_States (Class|BlackboardComponent|GetValueasEnum (Variables|Default|GetBlackboard) (Variables|Default|GetState%20Key)))))

(fn SetStateasPassive
  ;[0.15 0.15 0.15 0.5] Set Passive State
  (AI|Components|Blackboard|SetValueasEnum (Variables|Default|GetBlackboard) (Variables|Default|GetState%20Key) (Utilities|Enum|LiteralenumE_AI_States "NewEnumerator0")))

(fn SetStateasInvestigating
  (params (Location :type Vector))
  ;[0.15 0.15 0.15 0.5] Set State as investigating
  (AI|Components|Blackboard|SetValueasEnum (Variables|Default|GetBlackboard) (Variables|Default|GetState%20Key) (Utilities|Enum|LiteralenumE_AI_States "NewEnumerator2"))
  (AI|Components|Blackboard|SetValueasVector (Variables|Default|GetBlackboard) (Variables|Default|GetPoint%20Of%20Interest%20Key) Location))

(fn SetStateasTakingCover
  ;[0.15 0.15 0.15 0.5] Set Passive State
  (AI|Components|Blackboard|SetValueasEnum (Variables|Default|GetBlackboard) (Variables|Default|GetState%20Key) (Utilities|Enum|LiteralenumE_AI_States "NewEnumerator3")))

(fn SetStateasAttacking
  (params (Attack%20Target :type Actor%20Object%20Reference))
  ;[0.15 0.15 0.15 0.5] Set Attack Target
  (AI|Components|Blackboard|SetValueasObject (Variables|Default|GetBlackboard) (Variables|Default|GetAttack%20Target%20Key) Attack%20Target)
  ;[0.15 0.15 0.15 0.5] Set Passive State
  (AI|Components|Blackboard|SetValueasEnum (Variables|Default|GetBlackboard) (Variables|Default|GetState%20Key) (Utilities|Enum|LiteralenumE_AI_States "NewEnumerator1"))
  (Variables|Default|SetAttack%20Target Attack%20Target))

(fn CanSenseActor
  (params (Actor :type Actor%20Object%20Reference) (Sense :type E_AI_Sense%20Enum :default "NewEnumerator0"))
  ;[0.15 0.15 0.15 0.5] Can Sense Actor
  (bind _info (Class|AIPerceptionComponent|GetActorsPerception (Variables|Default|GetAIPerception) Actor))
  (for _array_element (.LastSensedStimuli (Utilities|Struct|BreakActorPerceptionBlueprintInfo _info))
    (bind _returnvalue (Class|AIPerceptionSystem|GetSenseClassforStimulus _array_element))
    (if (== _returnvalue (Utilities|Select :Index Sense :NewEnumerator0 0 :NewEnumerator1 "/Script/AIModule.AISense_Sight" :NewEnumerator2 "/Script/AIModule.AISense_Damage" :NewEnumerator3 0))
      (return (.bSuccessfullySensed (Utilities|Struct|BreakAIStimulus _array_element)) _array_element))))

(fn HandleSensedSight
  (params (Actor :type Actor%20Object%20Reference))
  ;[0.15 0.15 0.15 0.5] Handle sensed sight
  (bind _state (CallFunction|GetCurrentState))
  (switch Utilities|FlowControl|Switch|SwitchonE_AI_States _state
    (:NewEnumerator0
      _)
    (:NewEnumerator2
      _)
    (:NewEnumerator3
      _))
  (if (== Actor (Game|GetPlayerCharacter 0))
    (CallFunction|SetStateasAttacking Actor)))

(fn HandleSensedSound
  (params (Location :type Vector))
  ;[0.15 0.15 0.15 0.5] Handle Sensed Sound
  (bind _state (CallFunction|GetCurrentState))
  (switch Utilities|FlowControl|Switch|SwitchonE_AI_States _state
    (:NewEnumerator0
      _)
    (:NewEnumerator2
      _))
  (CallFunction|SetStateasInvestigating Location))

(fn HandleSensedDamage
  (params (Actor :type Actor%20Object%20Reference))
  ;[0.15 0.15 0.15 0.5] handle Damage
  (bind _state (CallFunction|GetCurrentState))
  (switch Utilities|FlowControl|Switch|SwitchonE_AI_States _state
    (:NewEnumerator0
      (CallFunction|SetStateasAttacking Actor))))