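; Match manager that runs the game timer and ends the round between the player and a single AI character.
; BeginPlay creates the HUD and end-screen widgets, caches both characters and starts the end timer.
; Tick updates the countdown and watches for a death.
; Either ending disables player input, stops AI logic and compares health to show win, loss or draw, but only time-up sets the GameInstance game-over flag.
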(event Custom|End%20Screen
  ;[1 0 0 0.5] Terminate game when time is up
  (if (Variables|Default|GetIs%20Time%20Up?)
    (CallFunction|TerminateAIandPlayerLogics)
    (CallFunction|CheckandDisplayResults)
    ;[0.15 0.15 0.15 0.5] Set 'Game Over' to TRUE
    (bind _asbp_game_instance (Utilities|Casting|CastToBP_GameInstance (Game|GetGameInstance)))
    (Variables|/Game/BLUEPRINTS/GameInstance/BP_GameInstance.BP_GameInstance_C|SetIs%20Game%20Over? _asbp_game_instance true)))

(event Custom|Check%20and%20Display%20Results
  ;[1 0 0 0.5] Display RESULT depending on health comparison
  (Utilities|Time|ClearandInvalidateTimerbyHandle (Variables|Default|GetGame%20Timer%20HDL))
  (Widget|RemovefromParent (Variables|Default|GetGameUI%20REF))
  (if (> (Variables|/Game/BLUEPRINTS/PlayerCharacter/BP_PlayerCharacter.BP_PlayerCharacter_C|GetCurrent%20Health (Variables|Default|GetPlayer%20REF)) (Variables|/Game/BLUEPRINTS/AICharacter/BP_AI_Character.BP_AI_Character_C|GetCurrent%20Health (Variables|Default|GetAI%20REF)))
    (Rendering|Components|TextRender|SetText (Variables|/Game/WIDGETS/GameUI/WBP_EndScreen.WBP_EndScreen_C|GetEndScreenText (Variables|Default|GetEnd%20Screen%20REF)) "YOU WIN :)")
    (UserInterface|Viewport|AddtoViewport (Variables|Default|GetEnd%20Screen%20REF) 0)
    (elif (> (Variables|/Game/BLUEPRINTS/AICharacter/BP_AI_Character.BP_AI_Character_C|GetCurrent%20Health (Variables|Default|GetAI%20REF)) (Variables|/Game/BLUEPRINTS/PlayerCharacter/BP_PlayerCharacter.BP_PlayerCharacter_C|GetCurrent%20Health (Variables|Default|GetPlayer%20REF)))
      (Rendering|Components|TextRender|SetText (Variables|/Game/WIDGETS/GameUI/WBP_EndScreen.WBP_EndScreen_C|GetEndScreenText (Variables|Default|GetEnd%20Screen%20REF)) "YOU LOST :(")
      (UserInterface|Viewport|AddtoViewport (Variables|Default|GetEnd%20Screen%20REF) 0)
      (elif (== (Variables|/Game/BLUEPRINTS/PlayerCharacter/BP_PlayerCharacter.BP_PlayerCharacter_C|GetCurrent%20Health (Variables|Default|GetPlayer%20REF)) (Variables|/Game/BLUEPRINTS/AICharacter/BP_AI_Character.BP_AI_Character_C|GetCurrent%20Health (Variables|Default|GetAI%20REF)))
        (Rendering|Components|TextRender|SetText (Variables|/Game/WIDGETS/GameUI/WBP_EndScreen.WBP_EndScreen_C|GetEndScreenText (Variables|Default|GetEnd%20Screen%20REF)) "DRAW")
        (UserInterface|Viewport|AddtoViewport (Variables|Default|GetEnd%20Screen%20REF) 0)))))

(event EventBeginPlay
  ;[0.15 0.15 0.15 0.5] Reference and add game UI to screen
  (bind _returnvalue (UserInterface|CreateWidget "/Game/WIDGETS/GameUI/WBP_GameUI.WBP_GameUI_C"))
  (bind _output_get (Variables|Default|SetGameUI%20REF _returnvalue))
  (UserInterface|Viewport|AddtoViewport _output_get 0)
  (Widget|SetVisibility _output_get "Collapsed")
  ;[0.15 0.15 0.15 0.5] Reference End Screen
  (bind _returnvalue_2 (UserInterface|CreateWidget "/Game/WIDGETS/GameUI/WBP_EndScreen.WBP_EndScreen_C"))
  (Variables|Default|SetEnd%20Screen%20REF _returnvalue_2)
  ;[0.15 0.15 0.15 0.5] Reference player
  (bind _asbp_player_character (Utilities|Casting|CastToBP_PlayerCharacter (Game|GetPlayerCharacter 0)))
  (Variables|Default|SetPlayer%20REF _asbp_player_character)
  ;[0.15 0.15 0.15 0.5] Reference AI character
  (bind _returnvalue_3 (Actor|GetActorOfClass "/Game/BLUEPRINTS/AICharacter/BP_AI_Character.BP_AI_Character_C"))
  (Variables|Default|SetAI%20REF _returnvalue_3)
  ;[0.15 0.15 0.15 0.5] Execute this once time is up
  (bind _returnvalue_4 (Utilities|Time|SetTimerbyEvent (delegate Custom|End%20Screen) (Variables|Default|GetGame%20Time)))
  (Variables|Default|SetGame%20Timer%20HDL _returnvalue_4))

(event EventTick
  (params (DeltaSeconds :type Float%20%28single-precision%29))
  (Utilities|FlowControl|Sequence
    (:then_0
      ;[0.15 0.15 0.15 0.5] Countdown as long as timer is active
      (if (Variables|Default|GetIs%20Timer%20Active?)
        ;[0.15 0.15 0.15 0.5] Game Time Countdown Logic
        (bind _output_get (Variables|Default|SetGame%20Time (Math|Float|Clamp(Float) (- (Variables|Default|GetGame%20Time) (Utilities|Time|GetWorldDeltaSeconds)) 0.0 (Variables|Default|GetGame%20Time))))
        (Rendering|Components|TextRender|SetText (Variables|/Game/WIDGETS/GameUI/WBP_GameUI.WBP_GameUI_C|GetTimer (Variables|Default|GetGameUI%20REF)) (Utilities|Text|ToText(String) (Class|KismetStringLibrary|TimeSecondstoString _output_get)))
        ;[0.15 0.15 0.15 0.5] Check if time is up
        (if (== (Variables|Default|GetGame%20Time) 0.0)
          (Variables|Default|SetIs%20Time%20Up? true))))
    (:then_1
      ;[0.15 0.15 0.15 0.5] Check if either of the characters is dead.
      (if (or (Variables|/Game/BLUEPRINTS/PlayerCharacter/BP_PlayerCharacter.BP_PlayerCharacter_C|GetIs%20Dead? (Variables|Default|GetPlayer%20REF)) (Variables|/Game/BLUEPRINTS/AICharacter/BP_AI_Character.BP_AI_Character_C|GetIs%20Dead? (Variables|Default|GetAI%20REF)))
        (Utilities|FlowControl|DoOnce false
          (:Completed
            (bind _output_get_2 (Variables|Default|SetIs%20Someone%20Dead? true))
            (if _output_get_2
              ;[1 0 0 0.5] Terminate game when someone is dead
              (Variables|Default|SetIs%20Timer%20Active? false)
              (CallFunction|TerminateAIandPlayerLogics)
              (CallFunction|CheckandDisplayResults))))))))

(fn ConstructionScript)

(fn TerminateAIandPlayerLogics
  (bind _returnvalue (Game|GetPlayerController 0))
  (bind _ai_ref (Variables|Default|GetAI%20REF))
  ;[1 0 0 0.5] Disable player input
  (Variables|/Script/Engine.PlayerController|SetbShowMouseCursor _returnvalue true)
  (Input|DisableInput (Game|GetPlayerCharacter 0) _returnvalue)
  ;[1 0 0 0.5] Terminate AI logic
  (bind _asbp_ai_controller (Utilities|Casting|CastToBP_AI_Controller (AI|GetAIController _ai_ref)))
  (AI|Logic|StopLogic (Variables|/Script/AIModule.AIController|GetBrainComponent _asbp_ai_controller) "Game Over")
  (Pawn|Components|CharacterMovement|DisableMovement (Variables|/Script/Engine.Character|GetCharacterMovement _ai_ref)))