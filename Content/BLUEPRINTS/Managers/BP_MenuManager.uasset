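; BP_MenuManager runs the game's main menu, creating the WBP_GameMenu widget over an infinitely looping level sequence with mouse input enabled.
; On BeginPlay it fades the menu in and reveals a skip button after a short delay.
; The menu content appears after a long timed wait, or earlier when the skip button is clicked, which fires once and hides the button.
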(event Custom|OnClicked_Event
  (bind _menu_ref (Variables|Default|GetMenu%20REF))
  (bind _menu_ref_2 (Variables|Default|GetMenu%20REF))
  ;[0.15 0.15 0.15 0.5] Show Menu Content
  (Utilities|FlowControl|DoOnce false
    (:Completed
      (Utilities|FlowControl|Sequence
        (:then_0
          (Widget|SetVisibility (Variables|/Game/WIDGETS/GameUI/WBP_GameMenu.WBP_GameMenu_C|GetSB_MenuContent _menu_ref_2) "SelfHitTestInvisible")
          (Default|ShowMenuContent _menu_ref_2)
          (Variables|Default|SetIs%20Menu%20Content%20Visible? true))
        (:then_1
          (Default|HideSkipButton _menu_ref)
          (Utilities|FlowControl|Delay 1.0)
          (Widget|SetVisibility (Variables|/Game/WIDGETS/GameUI/WBP_GameMenu.WBP_GameMenu_C|GetB_SkipIntro _menu_ref) "Hidden"))))))

(event EventBeginPlay
  (bind _returnvalue (Game|GetPlayerController 0))
  ;[0.15 0.15 0.15 0.5] Enable Input and show mouse cursor
  (Input|EnableInput _returnvalue)
  (Variables|/Script/Engine.PlayerController|SetbShowMouseCursor _returnvalue true)
  ;[0.15 0.15 0.15 0.5] Reference menu widget
  (bind _returnvalue_2 (UserInterface|CreateWidget "/Game/WIDGETS/GameUI/WBP_GameMenu.WBP_GameMenu_C"))
  (bind _output_get (Variables|Default|SetMenu%20REF _returnvalue_2))
  (UserInterface|Viewport|AddtoViewport _output_get 0)
  (Default|CinematicFadein _output_get)
  (Utilities|FlowControl|Sequence
    (:then_0
      ;[0.15 0.15 0.15 0.5] Play sequence and loop it infinitely
      (bind _returnvalue_3 (Sequencer|Player|CreateLevelSequencePlayer (Variables|Default|GetLevel%20Sequence)))
      (Class|MovieSceneSequencePlayer|PlayLooping _returnvalue_3 -1))
    (:then_1
      ;[0.15 0.15 0.15 0.5] Show skip button
      (Utilities|FlowControl|Delay 2.0)
      (Default|ShowSkipButton (Variables|Default|GetMenu%20REF))
      (EventDispatchers|AssignOnClicked (Variables|/Game/WIDGETS/GameUI/WBP_GameMenu.WBP_GameMenu_C|GetB_SkipIntro (Variables|Default|GetMenu%20REF)) (delegate Custom|OnClicked_Event))
      (if (not (Variables|Default|GetIs%20Menu%20Content%20Visible?))
        ;[0.15 0.15 0.15 0.5] Show Menu Buttons after 50 seconds
        (Utilities|FlowControl|Delay 5e+01)
        (Widget|SetVisibility (Variables|/Game/WIDGETS/GameUI/WBP_GameMenu.WBP_GameMenu_C|GetSB_MenuContent (Variables|Default|GetMenu%20REF)) "SelfHitTestInvisible")
        (Default|ShowMenuContent (Variables|Default|GetMenu%20REF))
        (Variables|Default|SetIs%20Menu%20Content%20Visible? true)))))

(fn ConstructionScript)